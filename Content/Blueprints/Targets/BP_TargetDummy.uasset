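; BP_TargetDummy is a shootable target actor that removes itself shortly after it spawns.
; BeginPlay starts a short delay that ends in DestroyActor, wired back into itself as a loop.
; Incoming damage lowers Health, and at zero the target spawns an NS_ImpactPoint effect at its skeletal mesh and destroys itself.
; That kill also increments the TargetsHit counter on the player's BP_FirstPersonCharacter.
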(event `self.ReceiveBeginPlay`
  ; Despawn Enemy
  (`KismetSystemLibrary.Delay` 2.0 :!label _label)
  (`self.K2_DestroyActor`)
  (goto _label))

(event `/Game/Core/Interfaces/BPI_Damageable.TakeDamage`
  (params (DamageAmount :type "Float (double-precision)"))
  (bind _skeletalmesh (`self.SkeletalMesh`))
  ; Enemy Take Damage
  (set `self.Health` (- (`self.Health`) DamageAmount))
  (if (<= (`self.Health`) 0.0)
    ; Bullet Impact Point
    (`NiagaraFunctionLibrary.SpawnSystemAtLocation` "/Game/Art/Niagara/NS_ImpactPoint.NS_ImpactPoint" (`SceneComponent.K2_GetComponentLocation` _skeletalmesh) (`SceneComponent.K2_GetComponentRotation` _skeletalmesh))
    (`self.K2_DestroyActor`)
    ; Targets Hit Count
    (bind _asbp_first_person_character (cast `/Game/FirstPerson/Blueprints/BP_FirstPersonCharacter` (`GameplayStatics.GetPlayerCharacter` 0)))
    (set `/Game/FirstPerson/Blueprints/BP_FirstPersonCharacter.TargetsHit` (+ (`/Game/FirstPerson/Blueprints/BP_FirstPersonCharacter.TargetsHit` _asbp_first_person_character) 1) _asbp_first_person_character)))

(fn `UserConstructionScript`)