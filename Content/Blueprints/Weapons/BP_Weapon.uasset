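; Hitscan weapon that handles firing, ammo, recoil and reloading, using a state check to gate shots.
; Fire spends ammo, plays muzzle effects and sound, then line traces from the supplied camera and sends damage through a message to the hit actor.
; A timeline offsets the weapon component for recoil, while dispatcher-style calls announce ammo changes and recoil requests.
; Reload switches state, waits on a fixed delay, then refills ammo.
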(event `PlayRecoil`
  ; Recoil
  (bind (_direction _recoilalpha) (`Timeline|RecoilTimeline` :!via `PlayFromStart`)
    (:`Update`
      (`SceneComponent.K2_SetRelativeLocation` (`self.weapon`) (+ (`self.OriginalWeaponLocation`) (* (`KismetMathLibrary.MakeVector` 0.0 0.0 -5.0) _recoilalpha)) false false))))

(event `self.ReceiveBeginPlay`
  ; SpawnWeapon
  (set `self.OriginalWeaponLocation` (`SceneComponent.RelativeLocation` (`self.weapon`))))

(event `Reload`
  ; Reloading
  (set `self.WeaponState` "NewEnumerator1")
  (`KismetSystemLibrary.Delay` 1.5)
  (set `self.CurrentAmmo` (`self.MaxAmmo`))
  (`self.AmmoChanged`)
  (set `self.WeaponState` "NewEnumerator0"))

(fn `Fire`
  (params (Camera :type "CameraComponent Object Reference"))
  (bind _returnvalue (`SceneComponent.K2_GetComponentLocation` Camera))
  (bind _muzzlepoint (`self.MuzzlePoint`))
  (if (`|EnumEquality` (`self.WeaponState`) "NewEnumerator0")
    (if (> (`self.CurrentAmmo`) 0)
      (set `self.CurrentAmmo` (- (`self.CurrentAmmo`) 1))
      (`self.AmmoChanged`)
      (`self.PlayRecoil`)
      (`self.RecoilRequested`)
      (`NiagaraFunctionLibrary.SpawnSystemAtLocation` "/Game/Art/Niagara/NS_MuzzleFlash.NS_MuzzleFlash" (`SceneComponent.K2_GetComponentLocation` _muzzlepoint) (`SceneComponent.K2_GetComponentRotation` _muzzlepoint))
      (`GameplayStatics.PlaySoundAtLocation` "/Game/Audio/freesound_community-9mm-pistol-shoot-short-reverb-7152.freesound_community-9mm-pistol-shoot-short-reverb-7152" (`SceneComponent.K2_GetComponentLocation` (`self.MuzzlePoint`)) (struct) 1.0 1.0 0.0 null null null null)
      (bind (_outhit _returnvalue_2) (`KismetSystemLibrary.LineTraceSingle` _returnvalue (+ _returnvalue (* (`SceneComponent.GetForwardVector` Camera) 5000.0)) "TraceTypeQuery1"))
      (if _returnvalue_2
        (message `/Game/Core/Interfaces/BPI_Damageable.TakeDamage` (`.HitActor` (`GameplayStatics.BreakHitResult` _outhit)) 25.0)))))

(fn `UserConstructionScript`)